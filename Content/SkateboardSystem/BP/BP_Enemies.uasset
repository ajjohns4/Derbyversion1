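; Roaming enemy, apparently a robot dog, that flashes a hurt widget and plays a defeat sound when the player overlaps its Hit component.
; AIMoveTo picks random reachable points, re-rolling on success.
; Tick and RandomSound share a randomly delayed chatter sound and brief bark widget.
; Also holds skateboard helpers for sphere physics, wheel traces, sockets and replicated montages, none called by the roaming logic.
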(event `random roam`
  (`|AIMoveTo` self (`NavigationSystemV1.K2_GetRandomReachablePointInRadius` (`self.K2_GetActorLocation`) 2500.0 null null) null
    (:`OnSuccess`
      (`self.random roam`))))

(event `self.ReceiveBeginPlay`
  (`|ExecutionSequence`
    (:`then_0`
      (`self.random roam`))
    (:`then_1`
      (`self.RandomSound`))))

(event `self.ReceiveTick`
  (params (DeltaSeconds :type "Float (single-precision)"))
  (`|ExecutionSequence` :!label _label
    (:`then_0`
      (`KismetSystemLibrary.Delay` (`KismetMathLibrary.RandomFloatInRange` 5.0 15.0))
      (`GameplayStatics.PlaySoundAtLocation` "/Game/DerbyAssets/Audio/RobotDogChatter.RobotDogChatter" (`SceneComponent.K2_GetComponentLocation` (`self.Mesh`)) (struct) 0.5 1.0 0.0 null null null null)
      (bind _returnvalue (`|CreateWidget` "/Game/UI/WipoutBark_WB.WipoutBark_WB_C"))
      (`UserWidget.AddToViewport` _returnvalue 0)
      (`KismetSystemLibrary.Delay` 1.0)
      (`Widget.RemoveFromParent` _returnvalue))))

(event `RandomSound`
  (goto _label))

(event `self.Hit.OnComponentBeginOverlap`
  (params (OverlappedComponent :type "PrimitiveComponent Object Reference") (OtherActor :type "Actor Object Reference") (OtherComp :type "PrimitiveComponent Object Reference") (OtherBodyIndex :type Integer) (bFromSweep :type Boolean) (SweepResult :type "HitResult Structure (by ref)"))
  (cast `/Game/ThirdPerson/Blueprints/BP_ThirdPersonCharacter` OtherActor)
  (`GameplayStatics.PlaySound2D` "/Game/DerbyAssets/Audio/RobotDogDefeat.RobotDogDefeat" 1.0 1.0 0.0 null null)
  (bind _returnvalue (`|CreateWidget` "/Game/UI/DerbyHurt_WB.DerbyHurt_WB_C" (`GameplayStatics.GetPlayerController` 0)))
  (`UserWidget.AddToViewport` _returnvalue 0)
  (`KismetSystemLibrary.Delay` 0.5)
  (`Widget.RemoveFromParent` _returnvalue))

(fn `GetLegPositions`
  (returns (FL :type "Vector Structure") (BL :type "Vector Structure"))
  (bind _skateboard (`self.skateboard`))
  (`/Engine/EditorBlueprintResources/StandardMacros.IsValid` _skateboard
    (:`Is Valid`
      (return (`SceneComponent.GetSocketLocation` _skateboard "FL") (`SceneComponent.GetSocketLocation` _skateboard "BL")))))

(fn `GetSimulatedVelocity`
  (returns (velocity :type "Vector Structure") (speed :type "Float (double-precision)"))
  (bind (_velocity _speed) (`self.GetSimulatedVelocityPure`))
  (return _velocity _speed))

(fn `GetSimulatedVelocityPure`
  (returns (velocity :type "Vector Structure") (speed :type "Float (double-precision)"))
  (bind _sim_sphere (`self.sim sphere`))
  (`/Engine/EditorBlueprintResources/StandardMacros.IsValid` _sim_sphere
    (:`Is Valid`
      (bind _returnvalue (`PrimitiveComponent.GetPhysicsLinearVelocity` _sim_sphere "None"))
      (return _returnvalue (`KismetMathLibrary.VSize` _returnvalue)))
    (:`Is Not Valid`
      (return (0.0 0.0 0.0) 0.0))))

(fn `GetUserInputs`
  (returns (`move forward` :type "Float (double-precision)") (`move right` :type "Float (double-precision)")))

(fn `Toggle Sim Sphere`
  (params (simulate :type Boolean))
  (bind _sim_sphere (`self.sim sphere`))
  (bind _sim_sphere_2 (`self.sim sphere`))
  (if simulate
    (`PrimitiveComponent.SetSimulatePhysics` _sim_sphere_2 true)
    (`PrimitiveComponent.AddImpulse` _sim_sphere_2 (* (`self.GetActorForwardVector`) 100000.0) "None" false)
    (else
      (`PrimitiveComponent.SetSimulatePhysics` _sim_sphere false)
      (`SceneComponent.K2_AttachToComponent` _sim_sphere null "None" "SnapToTarget" "SnapToTarget" "KeepWorld" true))))

(fn `UserConstructionScript`)

(fn `WheelTrace`
  (params (InputPin :type "Vector Structure"))
  (returns (`hit location` :type "Vector Structure") (Normal :type "Vector Structure") (`on ground` :type "Float (double-precision)"))
  (bind (_outhit _returnvalue) (`KismetSystemLibrary.LineTraceSingle` (+ InputPin (0.0 0.0 30.0)) (+ InputPin (0.0 0.0 -30.0)) "TraceTypeQuery2"))
  (if _returnvalue
    (bind (_bblockinghit _binitialoverlap _time _distance _location _impactpoint _normal) (`GameplayStatics.BreakHitResult` _outhit))
    (return _location _normal (`KismetMathLibrary.Conv_BoolToDouble` (< _distance 35.0)))
    (else
      (return InputPin (0.0 0.0 1.0) 0.0))))