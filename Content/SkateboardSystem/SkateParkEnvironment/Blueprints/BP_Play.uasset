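; BP_Play is an actor in the skate park environment that plays a media source through a media player.
; On BeginPlay, or when the StartPlayer event is called, it opens Source on Player, starts playback and turns looping on.
; The construction script also opens and plays the source, with looping off, so playback starts whenever the actor is constructed.
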(event `StartPlayer`
  (bind _player (`self.Player`))
  (`MediaPlayer.OpenSource` _player (`self.Source`) :!label _label)
  (`MediaPlayer.Play` _player)
  (`MediaPlayer.SetLooping` _player true))

(event `self.ReceiveBeginPlay`
  (goto _label))

(fn `UserConstructionScript`
  (bind _player (`self.Player`))
  (`MediaPlayer.OpenSource` _player (`self.Source`))
  (`MediaPlayer.Play` _player)
  (`MediaPlayer.SetLooping` _player false))