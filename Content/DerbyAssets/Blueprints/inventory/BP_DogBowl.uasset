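; BP_DogBowl is a collectible inventory item that counts toward the skateboard game mode's remaining collectables.
; PickUpItem decrements CollectablesLeft on GM_Skateboard, shows Collectible_WB, triggers the destroy event and returns the item.
; After a short delay, that event plays a collect sound at world origin, destroys the actor and adds DerbyHurt_WB.
; The widget's timed removal is sequenced after DestroyActor, on the destroyed actor.
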(event `Destoy item`
  (`KismetSystemLibrary.Delay` 0.1)
  (`GameplayStatics.PlaySoundAtLocation` "/Game/DerbyAssets/Audio/ItemCollect.ItemCollect" (0.0 0.0 0.0) (struct) 1.0 1.0 0.0 null null null null)
  (`self.K2_DestroyActor`)
  (bind _returnvalue (`|CreateWidget` "/Game/UI/DerbyHurt_WB.DerbyHurt_WB_C" (`GameplayStatics.GetPlayerController` 0)))
  (`UserWidget.AddToViewport` _returnvalue 0)
  (`KismetSystemLibrary.Delay` 1.0)
  (`Widget.RemoveFromParent` _returnvalue))

(fn `Pick up item`
  (returns (item :type String))
  (bind _asgm_skateboard (cast `/Game/SkateboardSystem/BP/GM_Skateboard` (`GameplayStatics.GetGameMode`)))
  (bind _result (`/Engine/EditorBlueprintResources/StandardMacros.DecrementInt` (`/Game/SkateboardSystem/BP/GM_Skateboard.Collectables left` _asgm_skateboard))
    (:`  `
      (set `/Game/SkateboardSystem/BP/GM_Skateboard.Collectables left` _result _asgm_skateboard)
      (bind _returnvalue (`|CreateWidget` "/Game/UI/Collectible_WB.Collectible_WB_C"))
      (`UserWidget.AddToViewport` _returnvalue 0)
      (`self.Destoy item`)
      (return (`self.item`)))))

(fn `UserConstructionScript`)