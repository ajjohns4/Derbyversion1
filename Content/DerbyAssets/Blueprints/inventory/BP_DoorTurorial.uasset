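; BP_DoorTurorial is the tutorial exit door that takes the player to the DerbyPark1 level.
; A Box overlap by BP_ThirdPersonCharacter enables input on the door so it can receive the E key.
; Pressing E works only when GM_Skateboard reports no collectables left, then swaps all widgets for a loading screen and opens the level after a short delay.
; End overlap calls DisableInput on the player controller rather than on the door.
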(event `Key|E`
  (params (Key :type "Key Structure"))
  (:`Pressed`
    (bind _asgm_skateboard (cast `/Game/SkateboardSystem/BP/GM_Skateboard` (`GameplayStatics.GetGameMode`)))
    (if (== (`/Game/SkateboardSystem/BP/GM_Skateboard.Collectables left` _asgm_skateboard) 0)
      (`GameplayStatics.PlaySound2D` "/Engine/VREditor/Sounds/UI/Gizmo_Handle_Clicked.Gizmo_Handle_Clicked" 1.0 1.0 0.0 null null)
      (`WidgetLayoutLibrary.RemoveAllWidgets`)
      (bind _returnvalue (`|CreateWidget` "/Game/UI/LoadingScreen_WB.LoadingScreen_WB_C" (`GameplayStatics.GetPlayerController` 0)))
      (`UserWidget.AddToViewport` _returnvalue 0)
      (`KismetSystemLibrary.Delay` 0.75)
      (`GameplayStatics.OpenLevel` "DerbyPark1"))))

(event `self.Box.OnComponentBeginOverlap`
  (params (OverlappedComponent :type "PrimitiveComponent Object Reference") (OtherActor :type "Actor Object Reference") (OtherComp :type "PrimitiveComponent Object Reference") (OtherBodyIndex :type Integer) (bFromSweep :type Boolean) (SweepResult :type "HitResult Structure (by ref)"))
  (cast `/Game/ThirdPerson/Blueprints/BP_ThirdPersonCharacter` OtherActor)
  (`self.EnableInput` (`GameplayStatics.GetPlayerController` 0)))

(event `self.Box.OnComponentEndOverlap`
  (params (OverlappedComponent :type "PrimitiveComponent Object Reference") (OtherActor :type "Actor Object Reference") (OtherComp :type "PrimitiveComponent Object Reference") (OtherBodyIndex :type Integer))
  (cast `/Game/ThirdPerson/Blueprints/BP_ThirdPersonCharacter` OtherActor)
  (`self.DisableInput` (`GameplayStatics.GetPlayerController` 0) null))

(fn `UserConstructionScript`)